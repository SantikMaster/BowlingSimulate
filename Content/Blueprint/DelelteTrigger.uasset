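; DelelteTrigger is a trigger volume that destroys any actor overlapping its BoxTrigger.
; If that actor derives from one of four Sphere classes, it sets a four-second timer calling NextMove on the player's FirstPersonCharacter.
; The Player1Turn toggle and the PlayerCounter score-table lookup are unconnected, and CallWid is empty.
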(event `self.BoxTrigger.OnComponentBeginOverlap`
  (params (OverlappedComponent :type "PrimitiveComponent Object Reference") (OtherActor :type "Actor Object Reference") (OtherComp :type "PrimitiveComponent Object Reference") (OtherBodyIndex :type Integer) (bFromSweep :type Boolean) (SweepResult :type "HitResult Structure (by ref)"))
  (bind _returnvalue (`GameplayStatics.GetPlayerCharacter` 0))
  (bind _returnvalue_2 (`GameplayStatics.GetObjectClass` OtherActor))
  (`self.K2_DestroyActor` OtherActor)
  (if (`KismetMathLibrary.ClassIsChildOf` _returnvalue_2 "/Game/Blueprint/Sphere_Class.Sphere_Class_C")
    (bind _asfirst_person_character (cast `/Game/FirstPersonCPP/Blueprints/FirstPersonCharacter` _returnvalue :!label _label))
    (`KismetSystemLibrary.K2_SetTimer` _returnvalue "NextMove" 4.0)
    (elif (`KismetMathLibrary.ClassIsChildOf` _returnvalue_2 "/Game/Blueprint/Sphere_Class_2.Sphere_Class_2_C")
      (goto _label)
      (elif (`KismetMathLibrary.ClassIsChildOf` _returnvalue_2 "/Game/Blueprint/Sphere_Class_3.Sphere_Class_3_C")
        (goto _label)
        (elif (`KismetMathLibrary.ClassIsChildOf` _returnvalue_2 "/Game/Blueprint/Sphere_Class_4.Sphere_Class_4_C")
          (goto _label))))))

(fn `CallWid`)

(fn `UserConstructionScript`)