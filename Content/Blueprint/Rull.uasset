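; Rull is a Blueprint of UI helper functions for score, strike and win feedback, with no active event logic of its own.
; TableEdit finds the first top-level PlayerCounter widget and calls PlayerScoreTable on it.
; StikeWid shows a StrikeWidget, while WinnerWid shows a WinWidget, reveals the mouse cursor and switches player 0 to UI-only input.
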(fn `StikeWid`
  (bind _returnvalue (`|CreateWidget` "/Game/UI/StrikeWidget.StrikeWidget_C" (`GameplayStatics.GetPlayerController` 0)))
  (`UserWidget.AddToViewport` _returnvalue 0))

(fn `TableEdit`
  (bind _foundwidgets (`WidgetBlueprintLibrary.GetAllWidgetsOfClass` "/Game/UI/PlayerCounter.PlayerCounter_C"))
  (bind _asplayer_counter (cast `/Game/UI/PlayerCounter` (`|GetArrayItem` _foundwidgets)))
  (`/Game/UI/PlayerCounter.PlayerScoreTable` _asplayer_counter))

(fn `UserConstructionScript`)

(fn `WinnerWid`
  (bind _returnvalue (`GameplayStatics.GetPlayerController` 0))
  (bind _returnvalue_2 (`|CreateWidget` "/Game/UI/WinWidget.WinWidget_C" _returnvalue))
  (`UserWidget.AddToViewport` _returnvalue_2 0)
  (set `PlayerController.bShowMouseCursor` true _returnvalue)
  (`WidgetBlueprintLibrary.SetInputMode_UIOnlyEx` _returnvalue _returnvalue_2))